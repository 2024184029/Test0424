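; Vest variant of the world item base Blueprint, representing a vest as an item placed in the world.
; InitSpawnData calls the parent, then looks up the spawn ID in DT_WorldItem_Vest to initialize item type, name, UI prefix and static mesh.
; The row also sets the mesh's rotation and scale, and the actor shifts along local Z by the mesh's bounds extent times a per-row factor.
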(fn `InitSpawnData`
  (params (ID :type Name) (SN :type String))
  (`parent.InitSpawnData` ID SN)
  (bind _returnvalue (`|GetDataTableRow` "/Game/Blueprints/Datas/DataTable/Item/DT_WorldItem_Vest.DT_WorldItem_Vest" (`self.ID`))
    (:`then`
      (`self.InitWorldItemBaseData` (break `/Game/Blueprints/Datas/Struct/Item/ST_WorldItem_Equipment` _returnvalue) (`.ItemName_5_539F961C4129FDAE41AB6AAC710A9354` (break `/Game/Blueprints/Datas/Struct/Item/ST_WorldItem_Equipment` _returnvalue)) (`.UIPrefix_8_E66149514DF4357F25AD0F878AF0C046` (break `/Game/Blueprints/Datas/Struct/Item/ST_WorldItem_Equipment` _returnvalue)) (`.StaticMesh_26_495E45CE45455F040C8807B357C2B07B` (break `/Game/Blueprints/Datas/Struct/Item/ST_WorldItem_Equipment` _returnvalue)))
      (`SceneComponent.K2_SetWorldRotation` (`self.StaticMesh`) (`.RotationOffset_17_249D7F074F431AB2F18645A739DB1070` (break `/Game/Blueprints/Datas/Struct/Item/ST_WorldItem_Equipment` _returnvalue)) false false)
      (`SceneComponent.SetWorldScale3D` (`self.StaticMesh`) (`.ScaleOffset_30_2412CAE94D8BEF0EB1A8E997164AA5A6` (break `/Game/Blueprints/Datas/Struct/Item/ST_WorldItem_Equipment` _returnvalue)))
      (`self.K2_AddActorLocalOffset` (`KismetMathLibrary.MakeVector` 0.0 0.0 (* (.z (`.BoxExtent` (`KismetSystemLibrary.GetComponentBounds` (`self.StaticMesh`)))) (`.BoundOffset_33_55C0653D4D1852539DE1E2B76F92A4B0` (break `/Game/Blueprints/Datas/Struct/Item/ST_WorldItem_Equipment` _returnvalue))))))))

(fn `UserConstructionScript`
  (`parent.UserConstructionScript`))