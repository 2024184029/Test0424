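; Player character Blueprint providing movement, look, free look, pose and move state, and walk speed functions.
; Free look decouples body yaw, keeps movement on the saved yaw, then a timeline lerps control rotation back by the shortest path on release.
; Move state resolves by overwriting in priority order: aim, walk, run, default jog.
; Tick only compares squared velocity to zero, firing a movement-state event on change.
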(event `self.ReceiveTick`
  (params (DeltaSeconds :type "Float (single-precision)"))
  (bind _returnvalue (> (`KismetMathLibrary.VSizeSquared` (`self.GetVelocity`)) 0.0))
  ; 단순 연산 (비교 등)만 할 것, 복잡연산은 X
  (if (!= (`self.bIsMovingNow`) _returnvalue)
    (bind _output_get (set `self.bIsMovingNow` _returnvalue))
    (`self.OnMovementStateChange` _output_get)))

(event `OnFreeLookEnded`
  ; 구현부
  (bind (_direction _alpha) (`Timeline|Timeline` :!via `PlayFromStart`)
    (:`Update`
      (`Controller.SetControlRotation` (`self.GetController`) (`KismetMathLibrary.RLerp` (`self.FreeLookEndRotation`) (`self.FreeLookStartRotation`) _alpha true)))
    (:`Finished`
      (set `self.bUseControllerRotationYaw` true))))

(fn `EvaluateMoveState`
  ; [우선순위]
  ; 조준 > 걷기 > 달리기 > 일반 조깅
  (`|ExecutionSequence`
    (:`then_0`
      (set `self.CurrentMoveState` "NewEnumerator1"))
    (:`then_1`
      (if (`self.bIsRunPressed`)
        (set `self.CurrentMoveState` "NewEnumerator2")))
    (:`then_2`
      (if (`self.bIsWalkPressed`)
        (set `self.CurrentMoveState` "NewEnumerator0")))
    (:`then_3`
      (if (`self.bIsAimPressed`)
        (set `self.CurrentMoveState` "NewEnumerator3")))))

(fn `FreeLook`
  (params (bIsPressed :type Boolean))
  (bind _returnvalue (`self.GetControlRotation`))
  (if bIsPressed
    ; FreeLook 시작 회전
    (set `self.FreeLookStartRotation` _returnvalue)
    (set `self.bUseControllerRotationYaw` false)
    (else
      ; FreeLook 끝났을 때 회전
      (set `self.FreeLookEndRotation` _returnvalue)
      ; 호출부
      (`self.OnFreeLookEnded`))))

(fn `GetMoveRotation`
  (returns (Result :type "Rotator Structure"))
  (return (`KismetMathLibrary.SelectRotator` (`/Game/Blueprints/Util/MathUtils.GetYawOnlyRotation` (`self.GetControlRotation`)) (`/Game/Blueprints/Util/MathUtils.GetYawOnlyRotation` (`self.FreeLookStartRotation`)) (`self.bUseControllerRotationYaw`))))

(fn `InputLookUp`
  (params (YAxis :type "Float (double-precision)"))
  (`self.AddControllerPitchInput` YAxis))

(fn `InputTurn`
  (params (XAxis :type "Float (double-precision)"))
  (`self.AddControllerYawInput` XAxis))

(fn `Move`
  (params (bIsForward :type Boolean) (AxisValue :type "Float (double-precision)"))
  (bind _result (`self.GetMoveRotation`))
  (if bIsForward
    (`self.AddMovementInput` (`KismetMathLibrary.GetForwardVector` _result) (`local.AxisValue`))
    (else
      (`self.AddMovementInput` (`KismetMathLibrary.GetRightVector` _result) (`local.AxisValue`)))))

(fn `SetMaxWalkSpeed`
  (params (NewSpeed :type "Float (double-precision)"))
  (set `CharacterMovementComponent.MaxWalkSpeed` NewSpeed (`self.CharacterMovement`)))

(fn `UpdateMoveState`
  (params (NewState :type "/Game/Blueprints/Datas/Enum/E_MoveState Enum" :default "NewEnumerator0"))
  (set `self.CurrentMoveState` NewState))

(fn `UpdatePoseState`
  (params (NewState :type "/Game/Blueprints/Datas/Enum/E_PoseState Enum" :default "NewEnumerator0"))
  (set `self.CurrentPoseState` NewState))

(fn `UserConstructionScript`)